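; BP_Room is a resizable modular room with switchable wall and floor materials, a fading grid and toggleable measurements.
; GenerateRoom, called on construction and from ChangeRoomDim's clamped resize, rebuilds floor, three walls, grid and measure lines as instanced meshes on 200-unit tiles, and updates the width label.
; RevealGrid drives grid opacity through a timeline into a Material Parameter Collection, and CloseGrid reverses it at a faster rate.
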(event `self.ReceiveBeginPlay`
  (`KismetMaterialLibrary.SetScalarParameterValue` "/Game/Materials/Misc/MPC_Grid.MPC_Grid" "Opacity"))

(event `RevealGrid`
  (`TimelineComponent.SetPlayRate` (`self.OpenGrid`) 0.1)
  (bind (_direction _opacity) (`Timeline|OpenGrid` :!via `PlayFromStart` :!label _label)
    (:`Update`
      (`KismetMaterialLibrary.SetScalarParameterValue` "/Game/Materials/Misc/MPC_Grid.MPC_Grid" "Opacity" _opacity))))

(event `CloseGrid`
  (`TimelineComponent.SetPlayRate` (`self.OpenGrid`) 1.0)
  (goto _label :!via `Reverse`))

(event `ShowMesures`
  (params (`Show?` :type Boolean))
  (`SceneComponent.SetVisibility` (`self.ISM_Mesure1`) `Show?` true)
  (`SceneComponent.SetVisibility` (`self.ISM_MesureZ`) `Show?` true)
  (set `self.ShowMesurements` `Show?`))

(event `ChangeWallsMaterial`
  (params (ElementIndex :type Integer))
  (`PrimitiveComponent.SetMaterial` (`self.ISM_Wall`) 0 (select `int` ElementIndex :`0` "/Game/Materials/WallMaterials/Mi_Wall_00.Mi_Wall_00" :`1` "/Game/Materials/WallMaterials/Mi_Wall_01.Mi_Wall_01" :`2` "/Game/Materials/WallMaterials/Mi_Wall_02.Mi_Wall_02" :!type "MaterialInterface Object Reference"))
  (set `self.WallMatIndex` ElementIndex))

(event `ChangeFloorMaterial`
  (params (ElementIndex :type Integer))
  (`PrimitiveComponent.SetMaterial` (`self.ISM_Floor`) 1 (select `int` ElementIndex :`0` "/Game/Materials/FloorMaterials/Mi_Floor00.Mi_Floor00" :`1` "/Game/Materials/FloorMaterials/Mi_Floor01.Mi_Floor01" :`2` "/Game/Materials/FloorMaterials/Mi_Floor02.Mi_Floor02" :!type "MaterialInterface Object Reference"))
  (set `self.FloorMatIndex` ElementIndex))

(fn `ChangeRoomDim`
  (params (X :type Integer) (Y :type Integer))
  (set `self.CountX` (`KismetMathLibrary.Clamp` (+ (`self.CountX`) X) 1 3))
  (set `self.CountY` (`KismetMathLibrary.Clamp` (+ (`self.CountY`) Y) 3 5))
  (`self.GenerateRoom` (`self.CountX`) (`self.CountY`)))

(fn `GenerateRoom`
  (params (X :type Integer) (Y :type Integer))
  (locals (YTileCount :type Integer) (XTileCount :type Integer))
  (bind _ytilecount (`local.YTileCount`))
  (bind _ytilecount_2 (`local.YTileCount`))
  (bind _ytilecount_3 (`local.YTileCount`))
  (bind _ytilecount_4 (`local.YTileCount`))
  (bind _ytilecount_5 (`local.YTileCount`))
  (set `local.XTileCount` (- X 1))
  (set `local.YTileCount` (- Y 1))
  (`InstancedStaticMeshComponent.ClearInstances` (`self.ISM_Floor`))
  (`InstancedStaticMeshComponent.ClearInstances` (`self.ISM_Wall`))
  (`InstancedStaticMeshComponent.ClearInstances` (`self.ISM_Grid`))
  (`InstancedStaticMeshComponent.ClearInstances` (`self.ISM_Mesure1`))
  (`|ExecutionSequence`
    (:`then_0`
      ;[1 1 1] Generate Back Wall
      (for _index (range (+ _ytilecount_2 1))
        (bind _returnvalue (- (`KismetMathLibrary.Conv_IntToDouble` (* _index 200)) (`KismetMathLibrary.SelectFloat` (* (/ _ytilecount_2 2) 250.0) (* (/ _ytilecount_2 2) 200) (> (mod (`local.YTileCount`) 2) 0))))
        (`InstancedStaticMeshComponent.AddInstance` (`self.ISM_Wall`) (`KismetMathLibrary.MakeTransform` (`KismetMathLibrary.MakeVector` (`KismetMathLibrary.Conv_IntToDouble` (* (`local.XTileCount`) 200)) _returnvalue) (struct :`Yaw` 180.0)) true)
        ;[1 1 1] Mesure Line
        (`InstancedStaticMeshComponent.AddInstance` (`self.ISM_Mesure1`) (`KismetMathLibrary.MakeTransform` (`KismetMathLibrary.MakeVector` 0.0 _returnvalue) (struct :`Yaw` 180.0)) true)))
    (:`then_1`
      ;[1 1 1] Generate Floor
      (for _index_2 (range (+ (`local.XTileCount`) 1))
        (for _index_3 (range (+ _ytilecount_3 1))
          (bind _returnvalue_2 (`KismetMathLibrary.Conv_IntToDouble` (* _index_2 200)))
          (bind _returnvalue_3 (- (`KismetMathLibrary.Conv_IntToDouble` (* _index_3 200)) (`KismetMathLibrary.SelectFloat` (* (/ _ytilecount_3 2) 250.0) (* (/ _ytilecount_3 2) 200) (> (mod (`local.YTileCount`) 2) 0))))
          (`InstancedStaticMeshComponent.AddInstance` (`self.ISM_Floor`) (`KismetMathLibrary.MakeTransform` (`KismetMathLibrary.MakeVector` _returnvalue_2 _returnvalue_3) (struct :`Yaw` 180.0)) true)
          ;[1 1 1] Generate Grid
          (`InstancedStaticMeshComponent.AddInstance` (`self.ISM_Grid`) (`KismetMathLibrary.MakeTransform` (`KismetMathLibrary.MakeVector` _returnvalue_2 _returnvalue_3) (struct :`Yaw` 180.0)) true))))
    (:`then_2`
      ;[1 1 1] Left side wall
      (for _index_4 (range (+ (`local.XTileCount`) 1))
        (bind _returnvalue_4 (`KismetMathLibrary.Conv_IntToDouble` (* _index_4 200)))
        (`InstancedStaticMeshComponent.AddInstance` (`self.ISM_Wall`) (`KismetMathLibrary.MakeTransform` (`KismetMathLibrary.MakeVector` _returnvalue_4 (`KismetMathLibrary.SelectFloat` (* (/ _ytilecount_5 2) -250.0) (* (/ _ytilecount_5 2) -200) (> (mod (`local.YTileCount`) 2) 0))) (struct :`Yaw` 90.0)) true)
        ;[1 1 1] Right Side Wall
        (`InstancedStaticMeshComponent.AddInstance` (`self.ISM_Wall`) (`KismetMathLibrary.MakeTransform` (`KismetMathLibrary.MakeVector` _returnvalue_4 (`KismetMathLibrary.SelectFloat` (* (/ _ytilecount 2) 350.0) (* (/ _ytilecount 2) 200) (> (mod (`local.YTileCount`) 2) 0))) (struct :`Yaw` -90.0)) true)))
    (:`then_3`
      (`TextRenderComponent.K2_SetText` (`self.TextRender`) (`KismetTextLibrary.Conv_StringToText` (`KismetStringLibrary.Concat_StrStr` (`KismetStringLibrary.Conv_IntToString` (* (+ (`local.YTileCount`) 1) 2)) " m.")))
      (`SceneComponent.K2_SetWorldLocation` (`self.ISM_MesureZ`) (`KismetMathLibrary.MakeVector` -200.0 (`KismetMathLibrary.SelectFloat` (- (* (/ _ytilecount_4 2) -250.0) 100.0) (- (* (/ _ytilecount_4 2) -200) 100.0) (> (mod (`local.YTileCount`) 2) 0)) 100.0) false false))))

(fn `UserConstructionScript`
  (`self.GenerateRoom` (`self.CountX`) (`self.CountY`)))