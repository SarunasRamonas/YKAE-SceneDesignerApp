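; Game instance that saves and loads named room designs for a furniture layout tool.
; SaveDesign stores room size, material indices, measurement visibility and each furniture's class, transform and material in an SG_Design slot per name.
; LoadDesign clears furniture, regenerates BP_Room and respawns saved pieces, passing WallIndex to the floor setter and FloorIndex to the walls.
; A separate "DList" slot tracks design names, rewritten on each add or remove.
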(event `SaveDesign`
  (params (DesignName :type String))
  (bind _returnvalue (`GameplayStatics.CreateSaveGameObject` "/Game/Blueprints/Core/SG_Design.SG_Design_C"))
  (bind _returnvalue_2 (`GameplayStatics.GetActorOfClass` "/Game/Blueprints/Core/BP_Room.BP_Room_C"))
  (set `/Game/Blueprints/Core/SG_Design.Save` (make `/Game/Blueprints/Core/Struct_SaveInfo` DesignName (`/Game/Blueprints/Core/BP_Room.CountX` _returnvalue_2) (`/Game/Blueprints/Core/BP_Room.CountY` _returnvalue_2) (`/Game/Blueprints/Core/BP_Room.WallMatIndex` _returnvalue_2) (`/Game/Blueprints/Core/BP_Room.FloorMatIndex` _returnvalue_2) (`/Game/Blueprints/Core/BP_Room.ShowMesurements` _returnvalue_2)) _returnvalue)
  (bind _outactors (`GameplayStatics.GetAllActorsOfClass` "/Game/Blueprints/Furniture/BP_FurnitureMaster.BP_FurnitureMaster_C"))
  (for _array_element _outactors
    (`KismetArrayLibrary.Array_Add` (`/Game/Blueprints/Core/SG_Design.FurnitureSaveInfo` _returnvalue) (make `/Game/Blueprints/Core/Struct_FurnitureSaveInfo` (`GameplayStatics.GetObjectClass` _array_element) (`Actor.GetTransform` _array_element) (make `/Game/Blueprints/Core/Struct_FurnitureData` (`/Game/Blueprints/Furniture/BP_FurnitureMaster.Material Index` _array_element)))))
  (`GameplayStatics.SaveGameToSlot` _returnvalue DesignName))

(event `LoadDesign`
  (params (DesignName :type String))
  (bind _outactors (`GameplayStatics.GetAllActorsOfClass` "/Game/Blueprints/Furniture/BP_FurnitureMaster.BP_FurnitureMaster_C"))
  (for _array_element _outactors
    (`Actor.K2_DestroyActor` _array_element))
  (bind _returnvalue (`GameplayStatics.LoadGameFromSlot` DesignName))
  (bind _assg_design (cast `/Game/Blueprints/Core/SG_Design` _returnvalue))
  (`self.GenerateRoomBySaveInfo` (`/Game/Blueprints/Core/SG_Design.Save` _assg_design))
  (for _array_element_2 (`/Game/Blueprints/Core/SG_Design.FurnitureSaveInfo` _assg_design)
    (bind (_furnitureclass _furnituretransform _saveinfo) (break `/Game/Blueprints/Core/Struct_FurnitureSaveInfo` _array_element_2))
    (bind _returnvalue_2 (`|SpawnActorFromClass` _furnitureclass _furnituretransform "Undefined" "OverrideRootScale" null null))
    (`/Game/Blueprints/Furniture/BP_FurnitureMaster.InitialSetup` _returnvalue_2 _saveinfo)))

(event `UpdateDesignNameList`
  (params (DesignName :type "String (by ref)") (`Add?` :type Boolean))
  (if `Add?`
    (`self.AddDesignNameToSaveList` DesignName)
    (else
      (`self.RemoveDesignNameInSaveList` DesignName))))

(event `LoadDesignList`
  (`self.LoadDesignNamesListOfSaveList`))

(fn `AddDesignNameToSaveList`
  (params (NewItem :type "String (by ref)"))
  (bind _designnames (`self.LoadDesignNamesListOfSaveList`))
  (bind _returnvalue (`GameplayStatics.CreateSaveGameObject` "/Game/Blueprints/Core/GS_DesignList.GS_DesignList_C"))
  (bind _output_get (set `/Game/Blueprints/Core/GS_DesignList.DesignNames` _designnames _returnvalue))
  (`KismetArrayLibrary.Array_Add` _output_get NewItem)
  (`GameplayStatics.SaveGameToSlot` _returnvalue "DList"))

(fn `GenerateRoomBySaveInfo`
  (params (Save :type "/Game/Blueprints/Core/Struct_SaveInfo Structure"))
  (bind (_designname _roomx _roomy _wallindex _floorindex _showmesurements) (break `/Game/Blueprints/Core/Struct_SaveInfo` Save))
  (bind _returnvalue (`GameplayStatics.GetActorOfClass` "/Game/Blueprints/Core/BP_Room.BP_Room_C"))
  (`/Game/Blueprints/Core/BP_Room.GenerateRoom` _returnvalue _roomx _roomy)
  (`/Game/Blueprints/Core/BP_Room.ChangeFloorMaterial` _returnvalue _wallindex)
  (`/Game/Blueprints/Core/BP_Room.ChangeWallsMaterial` _returnvalue _floorindex)
  (`/Game/Blueprints/Core/BP_Room.ShowMesures` _returnvalue _showmesurements))

(fn `LoadDesignNamesListOfSaveList`
  (returns (DesignNames :type "Array of String"))
  (bind _returnvalue (`GameplayStatics.LoadGameFromSlot` "DList"))
  (bind _asgs_design_list (cast `/Game/Blueprints/Core/GS_DesignList` _returnvalue))
  (return (`/Game/Blueprints/Core/GS_DesignList.DesignNames` _asgs_design_list)))

(fn `RemoveDesignNameInSaveList`
  (params (NewItem :type "String (by ref)"))
  (bind _designnames (`self.LoadDesignNamesListOfSaveList`))
  (bind _returnvalue (`GameplayStatics.CreateSaveGameObject` "/Game/Blueprints/Core/GS_DesignList.GS_DesignList_C"))
  (bind _output_get (set `/Game/Blueprints/Core/GS_DesignList.DesignNames` _designnames _returnvalue))
  (`KismetArrayLibrary.Array_RemoveItem` _output_get NewItem)
  (`GameplayStatics.SaveGameToSlot` _returnvalue "DList"))