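; Actor component that lets the mouse drag an actor around the world, showing a grab-hand hardware cursor during the grab.
; GrabStart stores the target actor, swaps the cursor and opens a Tick gate that line-traces from the deprojected cursor against one object type.
; On a hit, the actor moves to the impact point minus Offset.
; GrabEnd only restores the cursor; the gate is never closed.
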(event `self.ReceiveTick`
  (params (DeltaSeconds :type "Float (single-precision)"))
  (bind (_projectiontracestart _projectiontraceend) (`self.GetCursorLocationProjected` 1000))
  (`/Engine/EditorBlueprintResources/StandardMacros.Gate` true :!label _label
    (:`Exit`
      (bind (_outhit _returnvalue) (`KismetSystemLibrary.LineTraceSingleForObjects` _projectiontracestart _projectiontraceend (`|MakeArray` "ObjectTypeQuery7" :!type "EObjectTypeQuery Enum")))
      (if _returnvalue
        (`Actor.K2_SetActorLocation` (`self.GrabActor`) (- (`.ImpactPoint` (`GameplayStatics.BreakHitResult` _outhit)) (`self.Offset`)) false false)))))

(event `GrabStart`
  (params (GrabActor :type "/Game/Blueprints/Furniture/BP_FurnitureMaster Object Reference"))
  (set `self.GrabActor` GrabActor)
  (`self.SetGrabCursor` true)
  (goto _label :!via `Open`))

(event `GrabEnd`
  (`self.SetGrabCursor` false))

(fn `GetCursorLocationProjected`
  (params (ProjectionTraceAmount :type Integer))
  (returns (ProjectionTraceStart :type "Vector Structure") (ProjectionTraceEnd :type "Vector Structure"))
  (bind (_worldlocation _worlddirection) (`PlayerController.DeprojectMousePositionToWorld` (`GameplayStatics.GetPlayerController` 0)))
  (return _worldlocation (+ _worldlocation (* _worlddirection ProjectionTraceAmount))))

(fn `SetGrabCursor`
  (params (GrabCursor :type Boolean))
  (`WidgetBlueprintLibrary.SetHardwareCursor` (select `bool` GrabCursor :`false` "Default" :`true` "GrabHand" :!type "EMouseCursor Enum")))