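; Actor component for cursor-driven hover and selection of clickable world objects.
; Each tick it line-traces 1000 units along the deprojected mouse ray against the clickable object type.
; A new hit clears hover on all BI_CursorFunctions actors before sending hover-on to that actor; a miss clears hover.
; OnClicked_Event stores the hovered actor as SelectedObject and calls SelectedObjectUpdated; release is empty, and several leftover node chains never run.
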(event `self.ReceiveTick`
  (params (DeltaSeconds :type "Float (single-precision)"))
  (bind (_projectiontracestart _projectiontraceend) (`self.GetCursorLocationProjected` 1000))
  (`KismetSystemLibrary.Delay` 0.0)
  (bind (_outhit _returnvalue) (`KismetSystemLibrary.LineTraceSingleForObjects` _projectiontracestart _projectiontraceend (`self.ClickableObjectType`)))
  (if _returnvalue
    (bind (_bblockinghit _binitialoverlap _time _distance _location _impactpoint _normal _impactnormal _physmat _hitactor) (`GameplayStatics.BreakHitResult` _outhit))
    (`self.CompareOldHitActorWithNew` _hitactor
      (:`New`
        (bind _output_get (set `self.Hit Actor` _hitactor))
        (`self.UnHoverAllObjects`)
        (message `/Game/Blueprints/Core/Pawns/BI_CursorFunctions.OnCursorHoverOn` _output_get)))
    (else
      (`self.UnHoverObject`)
      (`self.UnHoverAllObjects`))))

(event `OnClicked_Event`
  (bind _output_get (set `self.SelectedObject` (`self.Hit Actor`)))
  (`self.SelectedObjectUpdated` _output_get))

(event `OnRelease_Event`)

(fn `DeselectObject`
  (set `self.SelectedObject` null)
  (return))

(fn `GetCursorLocationProjected`
  (params (ProjectionTraceAmount :type Integer))
  (returns (ProjectionTraceStart :type "Vector Structure") (ProjectionTraceEnd :type "Vector Structure"))
  (bind (_worldlocation _worlddirection) (`PlayerController.DeprojectMousePositionToWorld` (`GameplayStatics.GetPlayerController` 0)))
  (return _worldlocation (+ _worldlocation (* _worlddirection ProjectionTraceAmount))))

(fn `SelectObject`
  (params (SelectedObject :type "Actor Object Reference"))
  (set `self.SelectedObject` SelectedObject)
  (return))

(fn `UnHoverAllObjects`
  (bind _outactors (`GameplayStatics.GetAllActorsWithInterface` "/Game/Blueprints/Core/Pawns/BI_CursorFunctions.BI_CursorFunctions_C"))
  (for _array_element _outactors
    (message `/Game/Blueprints/Core/Pawns/BI_CursorFunctions.OnCursorHoverOff` _array_element)))

(fn `UnHoverObject`
  (bind _hit_actor (`self.Hit Actor`))
  (`/Engine/EditorBlueprintResources/StandardMacros.IsValid` _hit_actor
    (:`Is Valid`
      (message `/Game/Blueprints/Core/Pawns/BI_CursorFunctions.OnCursorHoverOff` _hit_actor)
      (set `self.Hit Actor` null))
    (:`Is Not Valid`
      _))
  (return))