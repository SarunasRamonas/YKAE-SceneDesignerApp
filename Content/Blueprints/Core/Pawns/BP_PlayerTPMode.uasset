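; Player pawn for a furniture placement mode, with a mouse-driven orbit camera and object manipulation.
; An intro rotation precedes input mapping, main widget creation and pitch limits; right-drag looks around, and scroll sets a clamped spring-arm zoom interpolated on Tick.
; ACObjectSelection feeds the selected furniture to the UI panel and to cursor dragging, rotation and deletion.
; Look input resets a timer for an optional idle yaw spin; Escape opens quit confirmation.
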(event `self.ReceiveBeginPlay`
  (bind _returnvalue (`GameplayStatics.GetPlayerCameraManager` 0))
  (bind _returnvalue_2 (`GameplayStatics.GetPlayerController` 0))
  (set `PlayerController.bShowMouseCursor` true (`GameplayStatics.GetPlayerController` 0))
  (`KismetSystemLibrary.Delay` 2.0)
  (`Timeline|InitialRotation` :!via `PlayFromStart`
    (:`Update`
      (`self.AddControllerPitchInput` 0.015)
      (`self.AddControllerYawInput` 0.05))
    (:`Finished`
      (`EnhancedInputSubsystemInterface.AddMappingContext` (pcsubsystem `EnhancedInputLocalPlayerSubsystem` _returnvalue_2) "/Game/Blueprints/PlayerInputMapping.PlayerInputMapping" 0 (struct))
      (`WidgetBlueprintLibrary.SetInputMode_GameAndUIEx` _returnvalue_2 null "DoNotLock" false)
      (bind _returnvalue_3 (`|CreateWidget` "/Game/Blueprints/UI/Widget_Main.Widget_Main_C"))
      (`UserWidget.AddToViewport` _returnvalue_3 0)
      (set `self.MainWidget` _returnvalue_3)
      (set `PlayerCameraManager.ViewPitchMin` -70.0 _returnvalue)
      (set `PlayerCameraManager.ViewPitchMax` 0.0 _returnvalue)
      (add `/Game/Blueprints/Core/Pawns/AC_ObjectSelection.SelectedObjectUpdated` (`self.AC_ObjectSelection`) (delegate `UpdateWidgetSelectedObjProperties`)))))

(event `UpdateWidgetSelectedObjProperties`
  (params (SelectedObject :type "Actor Object Reference"))
  (bind _asbp_furniture_master (cast `/Game/Blueprints/Furniture/BP_FurnitureMaster` SelectedObject :!pure true))
  (bind _mainwidget (`self.MainWidget`))
  (`/Engine/EditorBlueprintResources/StandardMacros.IsValid` SelectedObject
    (:`Is Valid`
      (`/Game/Blueprints/UI/Widget_Main.SetSelectedObjectPanelVisiblity` _mainwidget true)
      (if (not (`/Game/Blueprints/Furniture/BP_FurnitureMaster.IgnoreOverlapping` _asbp_furniture_master))
        (`/Game/Blueprints/UI/Widget_Main.UpdateSelectedObjectPanel` (`self.MainWidget`) _asbp_furniture_master))
      (set `self.SelectedObject` _asbp_furniture_master))
    (:`Is Not Valid`
      (`/Game/Blueprints/UI/Widget_Main.SetSelectedObjectPanelVisiblity` _mainwidget false)
      (set `self.SelectedObject` null))))

(event `ResetIdleAnimation`
  (bind _returnvalue (`KismetSystemLibrary.K2_SetTimerDelegate` (delegate `IdileAnimationStart`) 5.0 false 2.0 1.0 :!label _label))
  (set `self.IdleMovementTimer` _returnvalue))

(event `EnhancedInput|/Game/Blueprints/IA_Look`
  (params (ActionValue :type "Vector2D Structure") (ElapsedSeconds :type "Float (double-precision)") (TriggeredSeconds :type "Float (double-precision)") (InputAction :type "InputAction Object Reference" :default "/Game/Blueprints/IA_Look.IA_Look"))
  (:`Triggered`
    (`/Engine/EditorBlueprintResources/StandardMacros.Gate` true :!label _label_2
      (:`Exit`
        (`self.AddControllerYawInput` ActionValue_X)
        (`self.AddControllerPitchInput` (* ActionValue_Y -1.0))
        (`self.IdleAnimationEnd`)
        (goto _label)))))

(event `EnhancedInput|/Game/Blueprints/IA_Scroll`
  (params (ActionValue :type "Float (double-precision)") (ElapsedSeconds :type "Float (double-precision)") (TriggeredSeconds :type "Float (double-precision)") (InputAction :type "InputAction Object Reference" :default "/Game/Blueprints/IA_Scroll.IA_Scroll"))
  (:`Triggered`
    (set `self.Target Arm Length` (`SpringArmComponent.TargetArmLength` (`self.SpringArm`)))
    (set `self.NewArmLength` (+ (`self.Target Arm Length`) (* ActionValue -50.0)))
    (set `self.Alpha` 0.0)))

(event `Key|RightMouseButton`
  (params (Key :type "Key Structure"))
  (:`Pressed`
    (goto _label_2 :!via `Open`))
  (:`Released`
    (goto _label_2 :!via `Close`)))

(event `IdileAnimationStart`
  (if (`self.PlayIdleAnimation`)
    (bind _foundwidgets (`WidgetBlueprintLibrary.GetAllWidgetsOfClass` "/Game/Blueprints/UI/Widget_Main.Widget_Main_C"))
    (`/Game/Blueprints/UI/Widget_Main.Add message` (`|GetArrayItem` _foundwidgets) "Idle Animation")
    (`Timeline|Timeline` :!via `PlayFromStart` :!label _label_3
      (:`Update`
        (`self.AddControllerYawInput` 0.05)))))

(event `self.ReceiveTick`
  (params (DeltaSeconds :type "Float (single-precision)"))
  (set `SpringArmComponent.TargetArmLength` (`KismetMathLibrary.FClamp` (`KismetMathLibrary.Lerp` (`self.Target Arm Length`) (`self.NewArmLength`) (`self.Alpha`)) 250.0 500.0) (`self.SpringArm`))
  (set `self.Alpha` (`KismetMathLibrary.FClamp` (+ (`self.Alpha`) 0.1))))

(event `IdleAnimationEnd`
  (bind _foundwidgets (`WidgetBlueprintLibrary.GetAllWidgetsOfClass` "/Game/Blueprints/UI/Widget_Main.Widget_Main_C"))
  (if (> (`KismetArrayLibrary.Array_Length` _foundwidgets) 0)
    (`/Game/Blueprints/UI/Widget_Main.RemoveMessage` (`|GetArrayItem` _foundwidgets))
    (goto _label_3 :!via `Stop`)
    (else
      (goto _label_3 :!via `Stop`))))

(event `Key|Escape`
  (params (Key :type "Key Structure"))
  (:`Pressed`
    (bind _returnvalue (`|CreateWidget` "/Game/Blueprints/UI/Widget_ConfirmationQuit.Widget_ConfirmationQuit_C"))
    (`UserWidget.AddToViewport` _returnvalue 0)))

(event `Key|LeftMouseButton`
  (params (Key :type "Key Structure"))
  (bind _returnvalue (`GameplayStatics.GetPlayerController` 0))
  (bind _selectedobject (`self.SelectedObject`))
  (bind _selectedobject_2 (`self.SelectedObject`))
  (bind _ac_objectselection (`self.AC_ObjectSelection`))
  (:`Pressed`
    (`/Game/Blueprints/Core/Pawns/AC_ObjectSelection.OnClicked_Event` _ac_objectselection)
    (`/Engine/EditorBlueprintResources/StandardMacros.IsValid` _selectedobject_2
      (:`Is Valid`
        (`/Game/Blueprints/Furniture/BP_FurnitureMaster.MoveByCursorStart` _selectedobject_2)
        (set `PlayerController.CurrentMouseCursor` "GrabHandClosed" _returnvalue)
        (`self.IdleAnimationEnd`))))
  (:`Released`
    (`/Game/Blueprints/Core/Pawns/AC_ObjectSelection.OnRelease_Event` _ac_objectselection)
    (`/Engine/EditorBlueprintResources/StandardMacros.IsValid` _selectedobject
      (:`Is Valid`
        (`/Game/Blueprints/Furniture/BP_FurnitureMaster.MoveByCursorEnd` _selectedobject)
        (set `PlayerController.CurrentMouseCursor` "Default" _returnvalue)
        (`self.IdleAnimationEnd`)))))

(event `EnhancedInput|/Game/Blueprints/IA_Rotate`
  (params (ActionValue :type "Float (double-precision)") (ElapsedSeconds :type "Float (double-precision)") (TriggeredSeconds :type "Float (double-precision)") (InputAction :type "InputAction Object Reference" :default "/Game/Blueprints/IA_Rotate.IA_Rotate"))
  (bind _selectedobject (`self.SelectedObject`))
  (:`Triggered`
    (`/Engine/EditorBlueprintResources/StandardMacros.IsValid` _selectedobject
      (:`Is Valid`
        (`self.K2_AddActorLocalRotation` _selectedobject (`KismetMathLibrary.MakeRotator` 0.0 0.0 (* ActionValue 1.0)) false false)))))

(event `EnhancedInput|/Game/Blueprints/IA_Delete`
  (params (ActionValue :type "Float (double-precision)") (ElapsedSeconds :type "Float (double-precision)") (TriggeredSeconds :type "Float (double-precision)") (InputAction :type "InputAction Object Reference" :default "/Game/Blueprints/IA_Delete.IA_Delete"))
  (bind _selectedobject (`self.SelectedObject`))
  (:`Triggered`
    (`/Engine/EditorBlueprintResources/StandardMacros.IsValid` _selectedobject
      (:`Is Valid`
        (`/Game/Blueprints/Furniture/BP_FurnitureMaster.MoveByCursorEnd` _selectedobject)
        (`self.K2_DestroyActor` _selectedobject)))))

(fn `FurnitureSelected`
  (params (SelectedObject :type "/Game/Blueprints/Furniture/BP_FurnitureMaster Object Reference"))
  (set `self.SelectedObject` SelectedObject))

(fn `UserConstructionScript`)