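; Base furniture actor that the player drags across the floor with the cursor, with material switching.
; While the move gate is open, Tick traces from mouse to floor, optionally grid-snaps per the main widget's checkbox, and sweeps the actor, keeping its initial grab offset.
; Overlaps tint the mesh as an error through material scalars, and an overlapping release reverts to the starting location.
; Hover, selection and release highlights share a white-alpha parameter.
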(event `InitialSetup`
  (params (Struct_FurnitureData :type "/Game/Blueprints/Core/Struct_FurnitureData Structure (by ref)"))
  (`self.ChangeMaterial` (`.MaterialId_2_0A53AE33450B5B756B9B19AF39444444` (break `/Game/Blueprints/Core/Struct_FurnitureData` Struct_FurnitureData))))

(event `self.ReceiveTick`
  (params (DeltaSeconds :type "Float (single-precision)"))
  ;[0 0.04092 0.159] Core
  (`self.MoveByCursor`))

(event `self.FurnitureMesh.OnClicked`
  (params (TouchedComponent :type "PrimitiveComponent Object Reference") (ButtonPressed :type "Key Structure"))
  ;[0 0.04092 0.159] On Clicked
)

(event `MoveByCursor`
  (bind (_worldlocation _worlddirection) (`PlayerController.DeprojectMousePositionToWorld` (`GameplayStatics.GetPlayerController` 0)))
  ;[0 0.04092 0.159] Move by Cursor
  (`/Engine/EditorBlueprintResources/StandardMacros.Gate` true :!label _label
    (:`Exit`
      (bind (_outhit _returnvalue) (`KismetSystemLibrary.LineTraceSingleForObjects` _worldlocation (+ _worldlocation (* _worlddirection 1000)) (`|MakeArray` "ObjectTypeQuery7" :!type "EObjectTypeQuery Enum")))
      (if _returnvalue
        (if (`self.OffsetIsSet?`)
          (bind (_bblockinghit _binitialoverlap _time _distance _location _impactpoint) (`GameplayStatics.BreakHitResult` _outhit))
          (bind _returnvalue_2 (`KismetMathLibrary.SelectVector` (`KismetMathLibrary.MakeVector` (`KismetMathLibrary.GridSnap_Float` (.x _impactpoint) 10.0) (`KismetMathLibrary.GridSnap_Float` (.y _impactpoint) 10.0) (.z _impactpoint)) _impactpoint (`self.Snap`)))
          (`self.SetActorWorldLocationWithOffset` _returnvalue_2)
          (if (or (`self.Overlapping?`) (> (`KismetArrayLibrary.Array_Length` (`PrimitiveComponent.GetOverlappingActors` (`self.FurnitureMesh`) "/Game/Blueprints/Core/BP_Room.BP_Room_C")) 0))
            (`self.CollisionStart`)
            (else
              (`self.CollisionEnd`)))
          (else
            (set `self.Offset` (- _returnvalue_2 (`self.K2_GetActorLocation`)))
            (set `self.OffsetIsSet?` true)))))))

(event `MoveByCursorStart`
  (set `self.BeforeMovement` (`self.K2_GetActorLocation`))
  (set `self.Colliding` false)
  (set `self.LastPostion` false)
  ;[0 0.04092 0.159] Move by Cursor
  (set `self.OffsetIsSet?` false)
  (`/Game/Blueprints/Core/BF_Room.RevealGrid`)
  (`|ExecutionSequence`
    (:`then_0`
      (goto _label :!via `Open`))
    (:`then_1`
      (`self.SendToPlayer` self)
      (`self.IsSnapToTheGridNeeded`))
    (:`then_2`
      (`self.CollisionEnd`))))

(event `MoveByCursorEnd`
  ;[0 0.04092 0.159] Move by Cursor
  (`|ExecutionSequence`
    (:`then_0`
      (`/Game/Blueprints/Core/BF_Room.HideGrid`)
      (goto _label :!via `Close`))
    (:`then_1`
      (`self.OnCursorReleaseVisualEffect`))
    (:`then_2`
      (`KismetSystemLibrary.Delay` 0.01)
      (if (`self.Overlapping?`)
        (`self.K2_SetActorLocation` (`self.BeforeMovement`))
        (`self.CollisionEnd`)))))

(event `ChangeMaterial`
  (params (MaterialIndex :type Integer))
  (`PrimitiveComponent.SetMaterial` (`self.FurnitureMesh`) 0 (`|GetArrayItem` (`self.Materials`) MaterialIndex))
  (set `self.Material Index` MaterialIndex))

(event `/Game/Blueprints/Core/Pawns/BI_CursorFunctions.OnCursorHoverOn`
  (`MeshComponent.SetScalarParameterValueOnMaterials` (`self.FurnitureMesh`) "WhiteAlpha" 0.1))

(event `OnCursorReleaseVisualEffect`
  (bind (_direction _newtrack_0) (`Timeline|Timeline_0` :!via `PlayFromStart`)
    (:`Update`
      (`MeshComponent.SetScalarParameterValueOnMaterials` (`self.FurnitureMesh`) "WhiteAlpha" _newtrack_0))))

(event `/Game/Blueprints/Core/Pawns/BI_CursorFunctions.OnCursorHoverOff`
  (`MeshComponent.SetScalarParameterValueOnMaterials` (`self.FurnitureMesh`) "WhiteAlpha" 0.0))

(event `Selected`
  (bind _outactors (`GameplayStatics.GetAllActorsOfClass` "BP_FurnitureMaster_C"))
  (for _array_element _outactors
    (`MeshComponent.SetScalarParameterValueOnMaterials` (`/Game/Blueprints/Furniture/BP_FurnitureMaster.FurnitureMesh` _array_element) "WhiteAlpha" 0.0))
  (`MeshComponent.SetScalarParameterValueOnMaterials` (`self.FurnitureMesh`) "WhiteAlpha" 0.1))

(event `CollisionStart`
  (bind _furnituremesh (`self.FurnitureMesh`))
  (if (not (`self.IgnoreOverlapping`))
    (`MeshComponent.SetScalarParameterValueOnMaterials` _furnituremesh "ErrorAlpha" 1.0)
    (`MeshComponent.SetScalarParameterValueOnMaterials` _furnituremesh "WhiteAlpha" 0.5)
    (set `self.Colliding` true)))

(event `CollisionEnd`
  (bind _furnituremesh (`self.FurnitureMesh`))
  (if (not (`self.IgnoreOverlapping`))
    (`MeshComponent.SetScalarParameterValueOnMaterials` _furnituremesh "ErrorAlpha" 0.0)
    (`MeshComponent.SetScalarParameterValueOnMaterials` _furnituremesh "WhiteAlpha" 0.1)
    (set `self.Colliding` false)))

(fn `IsSnapToTheGridNeeded`
  (bind _foundwidgets (`WidgetBlueprintLibrary.GetAllWidgetsOfClass` "/Game/Blueprints/UI/Widget_Main.Widget_Main_C"))
  (set `self.Snap` (`CheckBox.IsChecked` (`/Game/Blueprints/UI/Widget_Main.Cb_SnapToGrid` (`|GetArrayItem` _foundwidgets)))))

(fn `Overlapping?`
  (returns (ReturnValue :type Boolean))
  (if (not (`self.IgnoreOverlapping`))
    (return (> (`KismetArrayLibrary.Array_Length` (`PrimitiveComponent.GetOverlappingActors` (`self.FurnitureMesh`) null)) 0))))

(fn `SendToPlayer`
  (params (SelectedObject :type "/Game/Blueprints/Furniture/BP_FurnitureMaster Object Reference"))
  (bind _asbp_player_tpmode (cast `/Game/Blueprints/Core/Pawns/BP_PlayerTPMode` (`GameplayStatics.GetPlayerPawn` 0)))
  (set `/Game/Blueprints/Core/Pawns/BP_PlayerTPMode.SelectedObject` SelectedObject _asbp_player_tpmode))

(fn `SetActorWorldLocationWithOffset`
  (params (`New WorldLocation` :type "Vector Structure"))
  (`self.K2_SetActorLocation` (- `New WorldLocation` (`self.Offset`)) true))

(fn `UserConstructionScript`)